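; Camera pawn that starts in CityView and handles touch look and animated transitions between named views.
; SetPawnView applies location, spring arm and FOV from CameraViewManager's view map.
; Touch drags rotate the spring arm, or dispatch horizontal distance during camera or card motion.
; Tick eases the camera with ExpoIn toward the target, then snaps to that view, with completion signaled at the start for CityView and at the end otherwise.
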(event `self.ReceiveBeginPlay`
  (`self.SetPawnView` "CityView")
  (`self.TransitionLevelCompleted` "CityView"))

(event `SetPawnView`
  (params (Key :type "ECameraView Enum" :default "ViewNone"))
  (bind _springarm (`self.SpringArm`))
  (bind (_value _returnvalue) (`BlueprintMapLibrary.Map_Find` (`/Game/BP/BP_CameraViewManager.ViewsToCameraTransform` (`self.CameraViewManager`)) Key))
  (bind (_cameraview _transform _springarmlenght _viewfield) (break `CameraViewInfo` _value))
  (bind _rotation (.rotation _transform))
  (if _returnvalue
    (`self.K2_SetActorLocation` (+ (.location _transform) (* (`KismetMathLibrary.GetForwardVector` _rotation) (`KismetMathLibrary.FTrunc` _springarmlenght))))
    (`SceneComponent.K2_SetRelativeRotation` _springarm _rotation false false)
    (set `SpringArmComponent.TargetArmLength` _springarmlenght _springarm)
    (set `CameraComponent.FieldOfView` _viewfield (`self.Camera`))
    (else
      (`KismetSystemLibrary.PrintString` "Error View"))))

(event `InputTouch`
  (params (Location :type "Vector Structure") (FingerIndex :type "ETouchIndex Enum"))
  ; 1. 视角旋转(包括俯仰)
  ; 2. 滑动游戏卡片(检测到卡片begin事件就禁用视角旋转)
  (:`Pressed`
    (set `self.StartLocation` Location)
    (set `self.LastLocation` Location))
  (:`Moved`
    (`|ExecutionSequence`
      (:`then_1`
        (if (or (`self.bCanMotion`) (`self.bCardMotion`))
          (`self.DispatchMoveDistance` (.x (- Location (`self.StartLocation`))))
          (else
            (`SceneComponent.K2_AddRelativeRotation` (`self.SpringArm`) (`KismetMathLibrary.MakeRotator` 0.0 (* (.y (- Location (`self.LastLocation`))) -0.1) (* (.x (- Location (`self.LastLocation`))) 0.1)) false false)
            (set `self.LastLocation` Location)))))))

(event `TransitionInterface.Transition2Target`
  (params (TargetView :type "ECameraView Enum" :default "ViewNone") (TargetPosition :type "Vector Structure"))
  (bind _camera (`self.Camera`))
  (bind _returnvalue (`SceneComponent.K2_GetComponentLocation` (`self.Camera`)))
  (if (`|EnumEquality` TargetView "CityView")
    (set `self.Target Position` (.location (`.Transform` (break `CameraViewInfo` (`BlueprintMapLibrary.Map_Find` (`/Game/BP/BP_CameraViewManager.ViewsToCameraTransform` (`self.CameraViewManager`)) "CityView")))))
    (set `self.TargetRotation` (.rotation (`.Transform` (break `CameraViewInfo` (`BlueprintMapLibrary.Map_Find` (`/Game/BP/BP_CameraViewManager.ViewsToCameraTransform` (`self.CameraViewManager`)) "CityView")))))
    (`SceneComponent.K2_SetWorldLocation` _camera (`self.LastTransitionPosition`) false false)
    (`SceneComponent.K2_SetWorldRotation` _camera (`self.LastTransitionRotation`) false false)
    (`self.TransitionLevelCompleted` "CityView")
    (else
      (set `self.Target Position` (+ _returnvalue (* (- TargetPosition _returnvalue) 0.9)))
      (set `self.TargetRotation` (`KismetMathLibrary.FindLookAtRotation` _returnvalue TargetPosition))))
  (set `self.CurrentTime` 0.0)
  (set `self.bCanMotion` true)
  (set `self.TargetView` TargetView))

(event `self.ReceiveTick`
  (params (DeltaSeconds :type "Float (single-precision)"))
  (bind _camera (`self.Camera`))
  (bind _targetview (`self.TargetView`))
  (bind _camera_2 (`self.Camera`))
  (if (`self.bCanMotion`)
    (bind _output_get (set `self.CurrentTime` (+ (/ DeltaSeconds 1.5) (`self.CurrentTime`))))
    (bind _result (`|EaseFunction` "ExpoIn" _output_get (`SceneComponent.K2_GetComponentLocation` _camera) (`self.Target Position`)))
    (`SceneComponent.K2_SetWorldLocation` _camera_2 _result false false)
    (set `self.LastTransitionPosition` _result)
    (bind _result_2 (`|EaseFunction` "ExpoIn" _output_get (`SceneComponent.K2_GetComponentRotation` _camera) (`self.TargetRotation`)))
    (`SceneComponent.K2_SetWorldRotation` _camera_2 _result_2 false false)
    (set `self.LastTransitionRotation` _result_2)
    (if (> _output_get (`KismetMathLibrary.SelectFloat` 1.0 0.65 (`|EnumEquality` (`self.TargetView`) "CityView")))
      (`SceneComponent.K2_SetRelativeRotation` :`self` _camera_2)
      (`SceneComponent.K2_SetRelativeLocation` _camera_2 (0.0 0.0 0.0) false false)
      (`self.SetPawnView` _targetview)
      (set `self.bCanMotion` false)
      (if (`|EnumInequality` _targetview "CityView")
        (`self.TransitionLevelCompleted` _targetview)))))

(event `SetTargetViewLight`
  (`/Game/BP/BP_SceneLightMgr.SwitchScene` (`self.SceneLightMgr`) (`self.TargetView`)))

(fn `UserConstructionScript`)