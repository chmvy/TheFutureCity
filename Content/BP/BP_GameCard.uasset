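; BP_GameCard is a touch-scrollable carousel of four card planes laid out along a spline.
; Touching its Box sets CardMotion on GM_Pawn, whose move-distance dispatcher drives ArrangeCard with the scaled drag offset.
; ArrangeCard spaces the planes evenly by spline time, aligns their rotation to the curve and enlarges those near the midpoint.
; The offset is clamped and saved when the touch leaves, so the next drag continues from there.
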(event `self.ReceiveBeginPlay`
  (bind _compcards (`self.CompCards`))
  (`KismetArrayLibrary.Array_Clear` (`self.CompCards`))
  (`KismetArrayLibrary.Array_Add` _compcards (`self.Plane0`))
  (`KismetArrayLibrary.Array_Add` _compcards (`self.Plane1`))
  (`KismetArrayLibrary.Array_Add` _compcards (`self.Plane2`))
  (`KismetArrayLibrary.Array_Add` _compcards (`self.Plane3`))
  (`self.ArrangeCard` 0.0)
  (bind _asgm_pawn (cast `/Game/GamePlay/GM_Pawn` (`GameplayStatics.GetPlayerPawn` 0)))
  (bind _output_get (set `self.As GM Pawn` _asgm_pawn))
  (add `/Game/GamePlay/GM_Pawn.DispatchMoveDistance` _output_get (delegate `DispatchMoveDistance_事件`)))

(event `DispatchMoveDistance_事件`
  (params (MoveDis :type "Float (double-precision)"))
  (`self.ArrangeCard` (/ MoveDis 1000.0)))

(event `ArrangeCard`
  (params (FirstCardPosition :type "Float (double-precision)"))
  (bind _spline (`self.Spline`))
  (bind _returnvalue (`KismetMathLibrary.FClamp` (+ FirstCardPosition (`self.CurrentFirstCardLocation`)) 0.0 0.5))
  (for (_array_element _array_index) (`self.CompCards`)
    (bind _returnvalue_2 (+ (* _array_index 0.166667) _returnvalue))
    (`SceneComponent.K2_SetWorldLocation` _array_element (`SplineComponent.GetLocationAtTime` _spline _returnvalue_2 "World" true) false false)
    (`SceneComponent.K2_SetRelativeRotation` _array_element (`KismetMathLibrary.MakeRotator` (+ (.roll (`SplineComponent.GetRotationAtTime` _spline _returnvalue_2 "Local" true)) 90.0) (.pitch (`SplineComponent.GetRotationAtTime` _spline _returnvalue_2 "Local" true)) (.yaw (`SplineComponent.GetRotationAtTime` _spline _returnvalue_2 "Local" true))) false false)
    (`SceneComponent.SetRelativeScale3D` _array_element (* (2.5 4.0 2.0) (`KismetMathLibrary.MapRangeClamped` (`KismetMathLibrary.Abs` (- _returnvalue_2 0.5)) 0.0 0.2 1.2 1.0))))
  (set `self.TempFirstCardLocation` _returnvalue))

(event `self.Box.OnInputTouchBegin`
  (params (FingerIndex :type "ETouchIndex Enum" :default "Touch1") (TouchedComponent :type "PrimitiveComponent Object Reference"))
  (bind _asgm_pawn (cast `/Game/GamePlay/GM_Pawn` (`GameplayStatics.GetPlayerPawn` 0)))
  (set `/Game/GamePlay/GM_Pawn.bCardMotion` true _asgm_pawn))

(event `self.Box.OnInputTouchLeave`
  (params (FingerIndex :type "ETouchIndex Enum" :default "Touch1") (TouchedComponent :type "PrimitiveComponent Object Reference"))
  (bind _asgm_pawn (cast `/Game/GamePlay/GM_Pawn` (`GameplayStatics.GetPlayerPawn` 0)))
  (set `/Game/GamePlay/GM_Pawn.bCardMotion` false _asgm_pawn)
  (set `self.CurrentFirstCardLocation` (`self.TempFirstCardLocation`)))

(fn `UserConstructionScript`)