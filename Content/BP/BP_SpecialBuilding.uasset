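; BP_SpecialBuilding is a tappable city landmark that shows a screen-space WBP_BuildingTag textured with its Appearance.
; Each tick it copies the camera's rotation and reprojects the tag above its Box component.
; Touching the Box broadcasts its CameraViewIndex and location to every TransitionInterface actor.
; Transition2Target shows the tag only in the city main scene view (城市主场景视角), collapsing it for other views.
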(event `self.ReceiveBeginPlay`
  (bind _returnvalue (`|CreateWidget` "/Game/WBP/BuildingTag/WBP_BuildingTag.WBP_BuildingTag_C"))
  (bind _output_get (set `self.TagWidget` _returnvalue))
  (`UserWidget.SetDesiredSizeInViewport` _output_get (300.0 180.0))
  (bind _aswbp_building_tag (cast `/Game/WBP/BuildingTag/WBP_BuildingTag` _output_get))
  (`/Game/WBP/BuildingTag/WBP_BuildingTag.SetTexture` _aswbp_building_tag (`self.Appearance`))
  (`UserWidget.AddToViewport` _output_get 0))

(event `self.Box.OnInputTouchBegin`
  (params (FingerIndex :type "ETouchIndex Enum" :default "Touch1") (TouchedComponent :type "PrimitiveComponent Object Reference"))
  (bind _outactors (`GameplayStatics.GetAllActorsWithInterface` "/Script/StageDemo.TransitionInterface"))
  (for _array_element _outactors
    (message `TransitionInterface.Transition2Target` _array_element (`self.CameraViewIndex`) (`SceneComponent.K2_GetComponentLocation` (`self.Box`)))))

(event `self.ReceiveTick`
  (params (DeltaSeconds :type "Float (single-precision)"))
  (`self.K2_SetActorRotation` (`PlayerCameraManager.GetCameraRotation` (`GameplayStatics.GetPlayerCameraManager` 0)))
  (`UserWidget.SetPositionInViewport` (`self.TagWidget`) (+ (`PlayerController.ProjectWorldLocationToScreen` (`GameplayStatics.GetPlayerController` 0) (`SceneComponent.K2_GetComponentLocation` (`self.Box`)) true) (-70.0 -120.0)) true))

(event `TransitionInterface.Transition2Target`
  (params (TargetView :type "ECameraView Enum" :default "ViewNone") (TargetPosition :type "Vector Structure"))
  (bind _tagwidget (`self.TagWidget`))
  (switch `ECameraView` TargetView
    (:`ViewNone`
      (`Widget.SetVisibility` _tagwidget "Collapsed" :!label _label))
    (:`CityView`
      (`Widget.SetVisibility` _tagwidget "Visible"))
    (:`ParkingView`
      (goto _label))
    (:`ChargeView`
      (goto _label))
    (:`GameView`
      (goto _label))))

(fn `UserConstructionScript`)