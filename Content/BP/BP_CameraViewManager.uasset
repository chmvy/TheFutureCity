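; Camera view manager that builds a lookup from each ECameraView enum value to a world transform taken from the level's CameraActors.
; CollecteCameraViews matches each camera's first actor tag against the enum names, storing hits in ViewsToCameraTransform and printing every non-matching comparison.
; On BeginPlay it only registers itself on the player's GM_Pawn; collection runs as a separate custom event.
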(event `CollecteCameraViews`
  (`KismetSystemLibrary.PrintString` "开始收集相机参数")
  (bind _outactors (`GameplayStatics.GetAllActorsOfClass` "/Script/Engine.CameraActor"))
  (for _array_element _outactors
    (bind _enumvalue (foreach `ECameraView` false)
      (:`LoopBody`
        (bind _returnvalue (`|GetEnumeratorName` _enumvalue))
        (bind _output (`|GetArrayItem` (`Actor.Tags` _array_element)))
        (if (== _returnvalue _output)
          (`BlueprintMapLibrary.Map_Add` (`self.ViewsToCameraTransform`) _enumvalue (make `CameraViewInfo` _enumvalue (`self.GetTransform` _array_element)))
          (else
            (`KismetSystemLibrary.PrintString` (`KismetStringLibrary.Concat_StrStr` (`KismetStringLibrary.Conv_NameToString` _returnvalue) "-----" (`KismetStringLibrary.Conv_NameToString` _output)))))))))

(event `self.ReceiveBeginPlay`
  (bind _asgm_pawn (cast `/Game/GamePlay/GM_Pawn` (`GameplayStatics.GetPlayerPawn` 0)))
  (set `/Game/GamePlay/GM_Pawn.CameraViewManager` self _asgm_pawn))

(fn `UserConstructionScript`)